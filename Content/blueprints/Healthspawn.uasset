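; Health pickup spawner that places a HealthItem inside its Box component's area.
; BeginPlay sets a single 15-second timer that calls spawnnewitem by name, with no looping or rescheduling shown.
; The event picks random X and Y within the box bounds, keeps Z at the box center, and spawns the item there.
; An unconnected rotation node using RotationSpeed never runs.
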(event Custom|spawnnewitem
  (bind _box (Variables|Default|GetBox))
  (bind (_origin _boxextent) (Collision|GetComponentBounds _box))
  (bind (_x _y _z) (Math|Vector|BreakVector _origin))
  (bind (_x_2 _y_2) (Math|Vector|BreakVector _boxextent))
  (Game|SpawnActorfromClass "/Game/blueprints/HealthItem.HealthItem_C" (Math|Conversions|ToTransform(Vector) (Math|Vector|MakeVector (Math|Random|RandomFloatinRange (- _x _x_2) (+ _x _x_2)) (Math|Random|RandomFloatinRange (- _y _y_2) (+ _y _y_2)) _z)) "Undefined" 0 0))

(event Collision|EventActorBeginOverlap
  (params (OtherActor :type Actor%20Object%20Reference)))

(event EventTick
  (params (DeltaSeconds :type Float%20%28single-precision%29)))

(event EventBeginPlay
  (Utilities|Time|SetTimerbyFunctionName 0 "spawnnewitem" 15.0))

(fn ConstructionScript)